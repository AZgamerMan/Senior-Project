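; Enemy turret Blueprint that sweeps its body on an idle timeline until anything overlaps its view cone, then tracks and fires at the player.
; The first overlap stops the sweep and changes the body material, with no reset shown.
; Tick turns body yaw and barrel pitch toward the player using interpolated rotation helpers.
; A self-restarting interval timeline repeatedly spawns projectiles from the barrel's socket.
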(event OnComponentBeginOverlap(Viewcone)
  (params (OverlappedComponent :type Primitive%20Component%20Object%20Reference) (OtherActor :type Actor%20Object%20Reference) (OtherComp :type Primitive%20Component%20Object%20Reference) (OtherBodyIndex :type Integer) (bFromSweep :type Boolean) (SweepResult :type Hit%20Result%20Structure%20%28by%20ref%29))
  ;[1 1 1] When Player seen, change Material, set Variable, and execute fire gun ONCE until reset
  (Variables|Default|SetPlayerVisible true)
  (Rendering|Material|SetMaterial (Variables|Default|GetTurret_Body) 1 "/Game/CustomContent/Enemies/turret_1/Materials/M_Turret_01_Light.M_Turret_01_Light")
  (Utilities|FlowControl|DoOnce false
    (:Completed
      (CallFunction|OnTargetFireGun)
      ;[1 1 1] Idle Animation
      (bind _newtrack_1 (Timeline|Timeline_0 Stop)
        (:Update
          (Transformation|SetRelativeRotation (Variables|Default|GetTurret_Body) (Math|Rotator|MakeRotator 0.0 0.0 _newtrack_1) false false))))))

(event Custom|OnTargetFireGun
  (bind _turret_barrel (Variables|Default|GetTurret_Barrel))
  (Timeline|FireProjectileInterval PlayFromStart
    (:Finished
      (Game|SpawnActorfromClass "/Game/CustomContent/Enemies/turret_1/BP_Turret_Projectile.BP_Turret_Projectile_C" (Math|Transform|MakeTransform (+ (Transformation|GetSocketLocation _turret_barrel "Projectile_Spawn") (* (Math|Vector|GetForwardVector _turret_barrel) 1e+01)) (Transformation|GetWorldRotation _turret_barrel)) "Undefined" 0 0)
      (CallFunction|OnTargetFireGun))))

(event EventTick
  (params (DeltaSeconds :type Float%20%28single-precision%29))
  (bind _returnvalue (Game|GetPlayerCharacter 0))
  (bind _turret_body (Variables|Default|GetTurret_Body))
  (bind _returnvalue_2 (Transformation|GetActorLocation _returnvalue))
  (bind _returnvalue_3 (Components|GetOwner _turret_body))
  (bind _returnvalue_4 (Transformation|GetActorLocation _returnvalue_3))
  (bind _returnvalue_5 (Math|Rotator|FindLookatRotation _returnvalue_4 _returnvalue_2))
  (bind _returnvalue_6 (|Body_Rotation _turret_body _returnvalue_5 DeltaSeconds))
  (if (Variables|Default|GetPlayerVisible)
    (Transformation|SetWorldRotation _turret_body _returnvalue_6 false false)
    (Transformation|SetWorldRotation (Variables|Default|GetTurret_Barrel) (|Barrel_Rotation DeltaSeconds _returnvalue_2 (.Yaw (Math|Rotator|BreakRotator _returnvalue_6))) false false)))

(event EventBeginPlay
  ;[1 1 1] Idle Animation
  (bind _newtrack_1 (Timeline|Timeline_0 Play)
    (:Update
      (Transformation|SetRelativeRotation (Variables|Default|GetTurret_Body) (Math|Rotator|MakeRotator 0.0 0.0 _newtrack_1) false false))))

(fn ConstructionScript)